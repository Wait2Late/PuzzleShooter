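; Parent Blueprint for numpad blocks, each showing a digit, C or a blank Backspace label on its Number widget, set from NumpadType at BeginPlay.
; C++-triggered events either perform an erasure or have BP_LevelManager check the password.
; Both paths then send messages to highlight the block's widget and update the player character's numbers.
; An older branch-based labelling version remains unconnected.
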(event `self.ReceiveBeginPlay`
  (bind _returnvalue (`KismetTextLibrary.Conv_IntToText` (`KismetMathLibrary.Conv_ByteToInt` (`self.NumpadType`))))
  (`self.Set Correct Text` (select `ENumpadType` (`self.NumpadType`) :`NumPad_0` _returnvalue :`NumPad_1` _returnvalue :`NumPad_2` _returnvalue :`NumPad_3` _returnvalue :`NumPad_4` _returnvalue :`NumPad_5` _returnvalue :`NumPad_6` _returnvalue :`NumPad_7` _returnvalue :`NumPad_8` _returnvalue :`NumPad_9` _returnvalue :`NumPad_C` (`KismetTextLibrary.Conv_StringToText` (`|GetEnumeratorNameAsString` (`self.NumpadType`))))))

(event `Only erase`
  ;[1 1 1] From C++ to update the UI
  (`self.C_Erasure`)
  (message `/Game/Blueprint/Interface/BPI_WidgetNumber.HighlightNumpad` (`WidgetComponent.GetWidget` (`self.Number`)) :!label _label)
  (message `/Game/Blueprint/Interface/BPI_PlayerEvents.UpdateNumbers` (`GameplayStatics.GetPlayerCharacter` 0)))

(event `self.UpdateNumberUI`
  ;[1 1 1] From C++ to update the UI
  (bind _returnvalue (`GameplayStatics.GetActorOfClass` "/Game/Blueprint/Manager/BP_LevelManager.BP_LevelManager_C"))
  (`/Game/Blueprint/Manager/BP_LevelManager.CheckPassword` _returnvalue)
  (goto _label))

(fn `Set Correct Text`
  (params (`Set new number` :type Text))
  (message `/Game/Blueprint/Interface/BPI_WidgetNumber.SetTextNumber` (`WidgetComponent.GetWidget` (`self.Number`)) `Set new number`))

(fn `UserConstructionScript`)