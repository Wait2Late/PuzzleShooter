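; Level manager that tracks puzzle level zones and decides when the current one is cleared.
; CheckPassword reads the DT_PuzzleLevels row indexed by the subsystem's current zone, validates its password and triggers LevelZoneCleared on success.
; When LevelZoneSubsystem signals a new zone, it waits briefly, erases the first number block found, then increments the zone and writes it back to the subsystem.
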(event `self.ReceiveBeginPlay`
  (add `LevelZoneSubsystem.OnNewLevelZoneReached` (subsystem `LevelZoneSubsystem`) (delegate `OnNewLevelZoneReached_Event`)))

(event `OnNewLevelZoneReached_Event`
  (bind _returnvalue (`GameplayStatics.GetActorOfClass` "/Game/Blueprint/NumPad/NumberBlocks/BP_NumberBlock_Parent.BP_NumberBlock_Parent_C"))
  (`KismetSystemLibrary.Delay` 0.5)
  (`/Game/Blueprint/NumPad/NumberBlocks/BP_NumberBlock_Parent.Only erase` _returnvalue)
  (bind _output_get (set `self.LevelZone` (cast `ELevelZoneType` (+ (`self.LevelZone`) 1))))
  (`LevelZoneSubsystem.SetLevelZone` (subsystem `LevelZoneSubsystem`) _output_get))

(event `CheckPassword`
  (bind _outrownames (`DataTableFunctionLibrary.GetDataTableRowNames` "/Game/DataTable/DT_PuzzleLevels.DT_PuzzleLevels"))
  (for _array_element _outrownames
    (bind _output (`|GetArrayItem` _outrownames (`KismetMathLibrary.Conv_ByteToInt` (`LevelZoneSubsystem.CurrentLevelZone` (subsystem `LevelZoneSubsystem`)))))
    (if (== _array_element _output)
      (bind _output_get (set `self.RowName` _output))
      (bind _returnvalue (`DataTableFunctionLibrary.DoesDataTableRowExist` "/Game/DataTable/DT_PuzzleLevels.DT_PuzzleLevels" _output_get))
      (if _returnvalue
        (bind _returnvalue_2 (`|GetDataTableRow` "/Game/DataTable/DT_PuzzleLevels.DT_PuzzleLevels" _output)
          (:`then`
            (bind (_levelzonetype _password) (break `PuzzleLevels` _returnvalue_2))
            (set `self.LevelZone` _levelzonetype)
            (bind _output_get_2 (set `self.Password` _password))
            (bind _returnvalue_3 (`self.IsPasswordValid` _output_get_2))
            (if _returnvalue_3
              (`LevelZoneSubsystem.TriggerLevelZoneCleared` (subsystem `LevelZoneSubsystem`))
              (break))))))))

(fn `UserConstructionScript`)