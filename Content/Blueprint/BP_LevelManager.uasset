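; BP_LevelManager is a level manager that checks puzzle passwords and advances the player through level zones.
; CheckPassword looks up the current zone's row in DT_PuzzleLevels by enum index and tests its Password.
; A valid password sends OpenDoorMessage with that zone to every BP_Door, then increments the zone and passes it to the GameInstance.
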(event `CheckPassword`
  (bind _output_get (set `self.LevelZone` (`self.LevelZone`)))
  (bind _outrownames (`DataTableFunctionLibrary.GetDataTableRowNames` "/Game/DataTable/DT_PuzzleLevels.DT_PuzzleLevels"))
  (for _array_element _outrownames
    (bind _output (`|GetArrayItem` _outrownames (`KismetMathLibrary.Conv_ByteToInt` _output_get)))
    (if (== _array_element _output)
      (bind _output_get_2 (set `self.RowName` _output))
      (bind _returnvalue (`DataTableFunctionLibrary.DoesDataTableRowExist` "/Game/DataTable/DT_PuzzleLevels.DT_PuzzleLevels" _output_get_2))
      (if _returnvalue
        (bind _returnvalue_2 (`|GetDataTableRow` "/Game/DataTable/DT_PuzzleLevels.DT_PuzzleLevels" _output)
          (:`then`
            (bind (_levelzonetype _password) (break `PuzzleLevels` _returnvalue_2))
            (set `self.LevelZone` _levelzonetype)
            (bind _output_get_3 (set `self.Password` _password))
            (bind _returnvalue_3 (`self.IsPasswordValid` _output_get_3))
            (if _returnvalue_3
              (bind _outactors (`GameplayStatics.GetAllActorsOfClass` "/Game/Blueprint/BP_Door.BP_Door_C"))
              (for _array_element_2 _outactors
                (message `/Game/Blueprint/Interface/BPI_InteractDoor.Open Door` _array_element_2 (`self.LevelZone`)))
              (bind _output_get_4 (set `self.LevelZone` (cast `ELevelZoneType` (+ (`self.LevelZone`) 1))))
              (message `GameInstanceInterface.SetLevelZone` (`GameplayStatics.GetGameInstance`) _output_get_4))))))))

(fn `UserConstructionScript`)